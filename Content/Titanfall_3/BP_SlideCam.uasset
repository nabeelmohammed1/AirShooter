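; BP_SlideCam is a camera modifier, apparently for a slide move, that eases a vertical offset and a field of view offset onto the view.
; Each update interpolates LiveZ and LiveFOV toward ZOffset and FOVOffset at the same speed, then adds them to the incoming height and FOV.
; The height output re-evaluates the interpolation on the updated LiveZ, so it runs one step ahead of the stored value.
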(fn `BlueprintModifyCamera`
  (params (DeltaTime :type "Float (single-precision)") (ViewLocation :type "Vector Structure") (ViewRotation :type "Rotator Structure") (FOV :type "Float (single-precision)"))
  (returns (NewViewLocation :type "Vector Structure") (NewViewRotation :type "Rotator Structure") (NewFOV :type "Float (single-precision)"))
  (bind _returnvalue (`KismetMathLibrary.FInterpTo` (`self.LiveZ`) (`self.ZOffset`) DeltaTime 10.0))
  (set `self.LiveZ` _returnvalue)
  (set `self.LiveFOV` (`KismetMathLibrary.FInterpTo` (`self.LiveFOV`) (`self.FOVOffset`) DeltaTime 10.0))
  (return (`KismetMathLibrary.MakeVector` ViewLocation_X ViewLocation_Y (+ ViewLocation_Z _returnvalue)) ViewRotation (+ FOV (`self.LiveFOV`))))