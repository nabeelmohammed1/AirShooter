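; GA_Sprint is a Gameplay Ability that makes the AirShooterCharacter sprint while the input is held.
; On activation it commits the ability, caches the current max walk speed, sets the sprint speed, and ends on input release.
; On end it restores the cached speed, removes effects granting the StaminaDrain tag, and prints an attribute value for debugging.
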(event `self.K2_ActivateAbility`
  (bind _charactermovement (`Character.CharacterMovement` (`self.Player`)))
  (`KismetSystemLibrary.PrintString` "sprint")
  (`self.K2_CommitAbility`)
  (bind _asair_shooter_character (cast `AirShooterCharacter` (`self.GetAvatarActorFromActorInfo`)))
  (set `self.Player` _asair_shooter_character)
  (set `self.Default Walk Speed` (`CharacterMovementComponent.MaxWalkSpeed` _charactermovement))
  (set `CharacterMovementComponent.MaxWalkSpeed` (`self.SprintSpeed`) _charactermovement)
  (`AbilityTask_WaitInputRelease.WaitInputRelease` false
    (:`OnRelease`
      (`self.K2_EndAbility`))))

(event `self.K2_OnEndAbility`
  (params (bWasCancelled :type Boolean))
  (set `CharacterMovementComponent.MaxWalkSpeed` (`self.Default Walk Speed`) (`Character.CharacterMovement` (`self.Player`)))
  (`self.BP_RemoveGameplayEffectFromOwnerWithGrantedTags` (struct :`GameplayTags` (struct :`(TagName` "Gameplay.Effect.StaminaDrain"))))
  (`KismetSystemLibrary.PrintString` (`KismetStringLibrary.Conv_DoubleToString` (`self.GetAttributeValue` (struct :`AttributeName` "Stamina" :`Attribute` "/Script/AirShooter.AirAttributes:Stamina" :`AttributeOwner` "/Script/CoreUObject.Class'/Script/AirShooter.AirAttributes'")))))