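; Gameplay ability that gives player 0 a jump and one directional double jump.
; Activation jumps from the ground or counts a fall as the first jump, then waits briefly before listening for another press.
; That press launches the character with a fixed vertical velocity, adding horizontal velocity from scaled momentum plus input direction boost.
; Returning to Walking ends the ability, which resets the jump count.
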(event `self.K2_OnEndAbility`
  (params (bWasCancelled :type Boolean))
  (set `self.JumpCount` 0))

(event `self.K2_ActivateAbility`
  (if (`NavMovementInterface.IsFalling` (`self.GetCharacterMovement`))
    (set `self.JumpCount` 1)
    (else
      (`Character.Jump` (`GameplayStatics.GetPlayerCharacter` 0))
      (`KismetSystemLibrary.PrintString` "1st Jump")
      (set `self.JumpCount` 1)))
  (`KismetSystemLibrary.Delay` 0.2)
  (`AbilityTask_WaitInputPress.WaitInputPress` false
    (:`then`
      (`AbilityTask_WaitMovementModeChange.CreateWaitMovementModeChange` "MOVE_Walking"
        (:`OnChange`
          (`KismetSystemLibrary.PrintString` "landed")
          (`self.K2_EndAbility`))))
    (:`OnPress`
      (if (< (`self.JumpCount`) 2)
        (`Character.LaunchCharacter` (`GameplayStatics.GetPlayerCharacter` 0) (`self.DirectionalJumping`) false true)
        (set `self.JumpCount` 2)
        (`KismetSystemLibrary.PrintString` "double jumped")
        (else
          (`KismetSystemLibrary.PrintString` "no 3td jump buddy" true true (struct :`R` 0.893212 :`G` 0.329236 :`B` 1.0 :`A` 1.0)))))))

(fn `DirectionalJumping`
  (returns (ReturnValue :type "Vector Structure"))
  (return (`KismetMathLibrary.MakeVector` (.x (+ (* (`MovementComponent.Velocity` (`self.GetCharacterMovement`)) (`self.KeepMomentum`)) (* (`PawnMovementComponent.GetLastInputVector` (`self.GetCharacterMovement`)) (`self.AirBoostStrenght`)))) (.y (+ (* (`MovementComponent.Velocity` (`self.GetCharacterMovement`)) (`self.KeepMomentum`)) (* (`PawnMovementComponent.GetLastInputVector` (`self.GetCharacterMovement`)) (`self.AirBoostStrenght`)))) (`self.DoubleJumpVel`))))