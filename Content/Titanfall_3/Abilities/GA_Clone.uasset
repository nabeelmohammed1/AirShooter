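; Gameplay ability that spawns two BP_CloneCharacter clones, one on each side of the avatar.
; On activation it commits, then chains two SpawnActor calls that offset along the avatar's right vector and turn each clone's yaw outward, with the avatar as instigator.
; The ability ends only when the second spawn succeeds; failed spawns just print debug text without ending it.
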(event `self.K2_ActivateAbilityFromEvent`
  (params (EventData :type "GameplayEventData Structure (by ref)"))
  (bind _returnvalue (`self.GetAvatarActorFromActorInfo`))
  (bind _returnvalue_2 (`Actor.K2_GetActorRotation` _returnvalue))
  (bind _returnvalue_3 (`Actor.K2_GetActorLocation` _returnvalue))
  (bind _asair_shooter_character (cast `AirShooterCharacter` (`self.GetAvatarActorFromActorInfo`) :!pure true))
  (bind _roll (.roll _returnvalue_2))
  (bind _pitch (.pitch _returnvalue_2))
  (bind _yaw (.yaw _returnvalue_2))
  (bind _returnvalue_4 (* (`KismetMathLibrary.GetRightVector` _returnvalue_2) 90.0))
  (`KismetSystemLibrary.PrintString` "clone start" true true (struct :`R` 1.0 :`G` 0.108445 :`B` 0.149841 :`A` 1.0))
  (`self.K2_CommitAbility`)
  (`GameplayTask_SpawnActor.SpawnActor` null (+ _returnvalue_3 _returnvalue_4) (`KismetMathLibrary.MakeRotator` _roll _pitch (+ _yaw 90.0)) "/Game/Titanfall_3/Pawns/BP_CloneCharacter.BP_CloneCharacter_C" false _asair_shooter_character
    (:`then`
      (`GameplayTask_SpawnActor.SpawnActor` null (- _returnvalue_3 _returnvalue_4) (`KismetMathLibrary.MakeRotator` _roll _pitch (- _yaw 90.0)) "/Game/Titanfall_3/Pawns/BP_CloneCharacter.BP_CloneCharacter_C" false _asair_shooter_character
        (:`Success`
          (`self.K2_EndAbility`))
        (:`DidNotSpawn`
          (`KismetSystemLibrary.PrintString` "failed x2" true true (struct :`R` 0.297868 :`G` 0.384913 :`B` 1.0 :`A` 1.0)))))
    (:`DidNotSpawn`
      (`KismetSystemLibrary.PrintString` "faiedx1" true true (struct :`R` 0.416408 :`G` 1.0 :`B` 0.314732 :`A` 1.0)))))