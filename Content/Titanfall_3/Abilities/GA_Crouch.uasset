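; Gameplay ability that crouches the player while input is held, turning the crouch into a slide at sprint speed.
; The slide temporarily swaps ground friction and braking, launches the character forward, and restores friction after a short delay.
; Both branches add a BP_SlideCam camera modifier, with a lower view and wider FOV for slides.
; Releasing input ends the ability, uncrouching, resetting movement and removing the modifier after easing offsets back.
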(event `self.K2_ActivateAbility`
  (`AbilityTask_WaitInputRelease.WaitInputRelease` false
    (:`then`
      (`self.FrictionStuff`)
      (if (> (`KismetMathLibrary.VSizeXY` (`MovementComponent.Velocity` (`self.GetCharacterMovement`))) 601.0)
        (`KismetSystemLibrary.PrintString` "sprint")
        (`Character.Crouch` (`GameplayStatics.GetPlayerCharacter` 0))
        (`self.SlideSetup`)
        (bind _returnvalue (`PlayerCameraManager.AddNewCameraModifier` (`GameplayStatics.GetPlayerCameraManager` 0) "/Game/Titanfall_3/BP_SlideCam.BP_SlideCam_C"))
        (bind _output_get (set `self.CamMod` _returnvalue))
        (set `/Game/Titanfall_3/BP_SlideCam.ZOffset` -60.0 _output_get)
        (set `/Game/Titanfall_3/BP_SlideCam.FOVOffset` 20.0 _output_get)
        (`Character.LaunchCharacter` (`GameplayStatics.GetPlayerCharacter` 0) (`self.SlideLaunch`) true false)
        (`AbilityTask_WaitDelay.WaitDelay` 0.7
          (:`OnFinish`
            (`self.ResetVals`)))
        (else
          (`KismetSystemLibrary.PrintString` "walk")
          (`Character.Crouch` (`GameplayStatics.GetPlayerCharacter` 0))
          (bind _returnvalue_2 (`PlayerCameraManager.AddNewCameraModifier` (`GameplayStatics.GetPlayerCameraManager` 0) "/Game/Titanfall_3/BP_SlideCam.BP_SlideCam_C"))
          (bind _output_get_2 (set `self.CamMod` _returnvalue_2))
          (set `/Game/Titanfall_3/BP_SlideCam.ZOffset` -15.0 _output_get_2)
          (set `/Game/Titanfall_3/BP_SlideCam.FOVOffset` 0.0 _output_get_2))))
    (:`OnRelease`
      (`self.K2_EndAbility`))))

(event `self.K2_OnEndAbility`
  (params (bWasCancelled :type Boolean))
  (bind _cammod (`self.CamMod`))
  (`Character.UnCrouch` (`GameplayStatics.GetPlayerCharacter` 0))
  (`self.ResetVals`)
  (set `CharacterMovementComponent.MaxWalkSpeed` 600.0 (`self.GetCharacterMovement`))
  (set `/Game/Titanfall_3/BP_SlideCam.ZOffset` 0.0 _cammod)
  (set `/Game/Titanfall_3/BP_SlideCam.FOVOffset` 0.0 _cammod)
  (`KismetSystemLibrary.Delay` 0.2)
  (`PlayerCameraManager.RemoveCameraModifier` (`GameplayStatics.GetPlayerCameraManager` 0) (`self.CamMod`)))

(fn `FrictionStuff`
  (bind _returnvalue (`self.GetCharacterMovement`))
  (set `self.OldGroundFriction` (`CharacterMovementComponent.GroundFriction` _returnvalue))
  (set `self.OldBrakingDecl` (`CharacterMovementComponent.BrakingDecelerationWalking` _returnvalue)))

(fn `ResetVals`
  (bind _returnvalue (`self.GetCharacterMovement`))
  (set `CharacterMovementComponent.GroundFriction` (`self.OldGroundFriction`) _returnvalue)
  (set `CharacterMovementComponent.BrakingDecelerationWalking` (`self.OldBrakingDecl`) _returnvalue))

(fn `SlideLaunch`
  (returns (SlideSpeed :type "Vector Structure"))
  (return (* (`Actor.GetActorForwardVector` (`self.GetAvatarActorFromActorInfo`)) 1200.0)))

(fn `SlideSetup`
  (bind _returnvalue (`self.GetCharacterMovement`))
  (set `CharacterMovementComponent.GroundFriction` (`self.NewFriction`) _returnvalue)
  (set `CharacterMovementComponent.BrakingDecelerationWalking` (`self.NewBrakingDecl`) _returnvalue))