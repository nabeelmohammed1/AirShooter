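; GA_Blink is an event-triggered gameplay ability that dashes the avatar with a short constant root motion force.
; The force's world direction is the raw hit location from the event's target data, or the avatar's location if that is zero.
; A Blink start gameplay cue plays until the ability ends when the force finishes.
; Finish mode maintains root motion velocity, though a clamp value from max movement speed is supplied.
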(event `self.K2_ActivateAbilityFromEvent`
  (params (EventData :type "GameplayEventData Structure (by ref)"))
  (bind (_bblockinghit _binitialoverlap _time _distance _location) (`GameplayStatics.BreakHitResult` (`AbilitySystemBlueprintLibrary.GetHitResultFromTargetData` (`.TargetData` (break `GameplayEventData` EventData)))))
  (`self.K2_CommitAbility`)
  (`AbilityTask_ApplyRootMotionConstantForce.ApplyRootMotionConstantForce` "None" (`KismetMathLibrary.SelectVector` (`Actor.K2_GetActorLocation` (`self.GetAvatarActorFromActorInfo`)) _location (== _location (0.0 0.0 0.0))) 2500.0 0.5 false null "MaintainLastRootMotionVelocity" (0.0 0.0 0.0) (`self.Get Velocity`)
    (:`then`
      (`self.K2_AddGameplayCue` (struct :`TagName` "GameplayCue.Blink.Start")))
    (:`OnFinish`
      (`self.K2_EndAbility`))))

(fn `Get Velocity`
  (returns (ReturnValue :type "Float (single-precision)"))
  (bind _aspawn (cast `Pawn` (`self.GetAvatarActorFromActorInfo`))
    (:`then`
      (return (`MovementComponent.GetMaxSpeed` (`Pawn.GetMovementComponent` _aspawn))))
    (:`CastFailed`
      (return 500.0))))