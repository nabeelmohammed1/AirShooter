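; Lobby character that represents a player with a tinted Quinn mesh, looping animation, info widget and VOIP.
; RepNotifies apply paint colour, server-picked random animation and player info, retrying on a timer until the widget is valid.
; A multicast registers the VOIP talker once PlayerState is valid.
; Holding H (positional) or J (radio) starts networked voice and sets the replicated voice mode, which switches talker settings.
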(event `RandomAnm`
  (`KismetSystemLibrary.Delay` 0.5)
  (`/Engine/EditorBlueprintResources/ActorMacros.Switch Has Authority`
    (:`Authority`
      (set `self.AnimIndex` (`.OutIndex` (`KismetArrayLibrary.Array_Random` (`self.LobbyAnims`)))))))

(event `self.ReceiveBeginPlay`
  (bind _returnvalue (`KismetMaterialLibrary.CreateDynamicMaterialInstance` "/Game/Titanfall_3/Mats/MI_Overlay.MI_Overlay" "Colour"))
  (set `self.MatInst` _returnvalue))

(event `Play Anim`
  (params (NewAnimToPlay :type "AnimationAsset Object Reference"))
  (`SkeletalMeshComponent.PlayAnimation` (`self.Mesh`) NewAnimToPlay true))

(event `Mulitcast_InitVOIP`
  (bind _playerstate (`self.PlayerState`))
  (`KismetSystemLibrary.PrintString` "voice" true true (struct :`R` 1.0 :`G` 0.397696 :`B` 0.827474 :`A` 1.0))
  (`/Engine/EditorBlueprintResources/StandardMacros.IsValid` _playerstate :!label _label
    (:`Is Valid`
      (`AdvancedVoiceLibrary.RemoveAllRemoteTalkers`)
      (`VOIPTalker.RegisterWithPlayerState` (`self.VOIPTalker`) _playerstate)
      (`VOIPStatics.SetMicThreshold` -1.5)
      (set `VOIPTalker.Settings` (select `/Game/Titanfall_3/Data/E_VoiceMode` (`self.voiceMode`) :`NewEnumerator0` (make `VoiceSettings` null) :`NewEnumerator1` (make `VoiceSettings` (`self.Mesh`) "/Game/Titanfall_3/Data/SA_Positional.SA_Positional") :`NewEnumerator2` (make `VoiceSettings` null)) (`self.VOIPTalker`)))
    (:`Is Not Valid`
      (`KismetSystemLibrary.RetriggerableDelay` 0.2)
      (goto _label))))

(event `Server_SetVoiceMode`
  (params (voiceMode :type "/Game/Titanfall_3/Data/E_VoiceMode Enum" :default "NewEnumerator0"))
  (set `self.voiceMode` voiceMode))

(event `Key|H`
  (params (Key :type "Key Structure"))
  (:`Pressed`
    (`self.VOIPTalker`
      (:`then`
        (`self.Server_SetVoiceMode` "NewEnumerator1")
        (`AdvancedVoiceLibrary.StartNetworkedVoice` 0)
        (`KismetSystemLibrary.ExecuteConsoleCommand` "OSS.VoiceLoopback 1" (`PlayerState.GetPlayerController` (`self.PlayerState`)))
        (`KismetSystemLibrary.PrintString` "start'" true true (struct :`R` 1.0 :`G` 0.907213 :`A` 1.0)))
      (:`else`)))
  (:`Released`
    (`AdvancedVoiceLibrary.StopNetworkedVoice` 0)
    (`self.Server_SetVoiceMode` "NewEnumerator0")))

(event `Key|J`
  (params (Key :type "Key Structure"))
  (:`Pressed`
    (`self.VOIPTalker`
      (:`then`
        (`self.Server_SetVoiceMode` "NewEnumerator2")
        (`AdvancedVoiceLibrary.StartNetworkedVoice` 0))
      (:`else`)))
  (:`Released`
    (`AdvancedVoiceLibrary.StopNetworkedVoice` 0)
    (`self.Server_SetVoiceMode` "NewEnumerator0")))

(event `Client_CloseVoiceLine`
  (`self.VOIPTalker`
    (:`then`
      (if (`|EnumInequality` (`self.voiceMode`) "NewEnumerator0")
        (`KismetSystemLibrary.ExecuteConsoleCommand` "ToggleSpeaking 0" (`PlayerState.GetPlayerController` (`self.PlayerState`))))
      (`AdvancedVoiceLibrary.MuteRemoteTalker` 0 (`AdvancedSessionsLibrary.GetUniqueNetIDFromPlayerState` (`self.PlayerState`)) true)
      (`AdvancedVoiceLibrary.RemoveAllRemoteTalkers`)
      (`VOIPLibrary.ClearVoicePackets` self))
    (:`else`)))

(event `self.ReceiveUnpossessed`
  (params (OldController :type "Controller Object Reference")))

(fn `OnRep_AnimIndex`
  (`self.Play Anim` (`|GetArrayItem` (`self.LobbyAnims`) (`self.AnimIndex`))))

(fn `OnRep_ColourVal`
  (bind _colourval (`self.ColourVal`))
  (bind _mesh (`self.Mesh`))
  (bind _returnvalue (`PrimitiveComponent.CreateDynamicMaterialInstance` _mesh 0 "/Game/Characters/Mannequins/Materials/Quinn/MI_Quinn_01.MI_Quinn_01" "None"))
  (bind _returnvalue_2 (`PrimitiveComponent.CreateDynamicMaterialInstance` _mesh 1 "/Game/Characters/Mannequins/Materials/Quinn/MI_Quinn_02.MI_Quinn_02" "None"))
  (`MaterialInstanceDynamic.SetVectorParameterValue` _returnvalue "Paint Tint" _colourval)
  (`MaterialInstanceDynamic.SetVectorParameterValue` _returnvalue_2 "Paint Tint" _colourval))

(fn `OnRep_playerInfo`
  (bind _returnvalue (`WidgetComponent.GetWidget` (`self.Widget`)))
  (`/Engine/EditorBlueprintResources/StandardMacros.IsValid` _returnvalue
    (:`Is Valid`
      (bind _aswbp_player_lobby_info (cast `/Game/Titanfall_3/GameData/LobbyGamemode/LobbyData/WBP_PlayerLobbyInfo` _returnvalue))
      (`/Game/Titanfall_3/GameData/LobbyGamemode/LobbyData/WBP_PlayerLobbyInfo.UpdatePlayerInfo` _aswbp_player_lobby_info (`self.playerInfo`))
      (`SceneComponent.SetVisibility` (`self.Widget`) true false)
      (`KismetSystemLibrary.PrintString` "ui wya"))
    (:`Is Not Valid`
      (`KismetSystemLibrary.K2_SetTimer` null "OnRep_playerInfo" 0.1))))

(fn `OnRep_voiceMode`
  (set `VOIPTalker.Settings` (select `/Game/Titanfall_3/Data/E_VoiceMode` (`self.voiceMode`) :`NewEnumerator0` (make `VoiceSettings` null) :`NewEnumerator1` (make `VoiceSettings` (`self.Mesh`) "/Game/Titanfall_3/Data/SA_Positional.SA_Positional") :`NewEnumerator2` (make `VoiceSettings` null)) (`self.VOIPTalker`)))

(fn `UpdatePlayerInfo`
  (params (playerInfo :type "/Game/Titanfall_3/GameData/LobbyGamemode/LobbyData/S_PlayerLobbyInfo Structure"))
  (set `self.playerInfo` playerInfo)
  (`KismetSystemLibrary.PrintString` "updqted"))

(fn `UserConstructionScript`
  (bind _colourval (`self.ColourVal`))
  (bind _mesh (`self.Mesh`))
  (bind _returnvalue (`PrimitiveComponent.CreateDynamicMaterialInstance` _mesh 0 "/Game/Characters/Mannequins/Materials/Quinn/MI_Quinn_01.MI_Quinn_01" "None"))
  (bind _returnvalue_2 (`PrimitiveComponent.CreateDynamicMaterialInstance` _mesh 1 "/Game/Characters/Mannequins/Materials/Quinn/MI_Quinn_02.MI_Quinn_02" "None"))
  (`MaterialInstanceDynamic.SetVectorParameterValue` _returnvalue "Paint Tint" _colourval)
  (`MaterialInstanceDynamic.SetVectorParameterValue` _returnvalue_2 "Paint Tint" _colourval))