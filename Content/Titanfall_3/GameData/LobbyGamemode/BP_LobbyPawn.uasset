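; Lobby pawn that provides push-to-talk voice chat, with H for positional voice and J for radio.
; Keys set a server-side VoiceMode, whose OnRep swaps VOIP talker settings between attached, attenuated audio and non-spatial defaults.
; A multicast init retries until PlayerState is valid, then registers the talker.
; Unpossess mutes and clears voice, while voice loopback is switched on at BeginPlay and on H.
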(event `self.ReceiveBeginPlay`
  (`KismetSystemLibrary.ExecuteConsoleCommand` "OSS.VoiceLoopback 1" null)
  (`self.Server_SetVoiceMode` "NewEnumerator1"))

(event `Mulitcast_InitVOIP`
  (bind _playerstate (`self.PlayerState`))
  (`KismetSystemLibrary.PrintString` "voice" true true (struct :`R` 1.0 :`G` 0.397696 :`B` 0.827474 :`A` 1.0))
  (`/Engine/EditorBlueprintResources/StandardMacros.IsValid` _playerstate :!label _label
    (:`Is Valid`
      (`AdvancedVoiceLibrary.RemoveAllRemoteTalkers`)
      (`VOIPTalker.RegisterWithPlayerState` (`self.VOIPTalker`) _playerstate)
      (`VOIPStatics.SetMicThreshold` -1.5)
      (set `VOIPTalker.Settings` (select `/Game/Titanfall_3/Data/E_VoiceMode` (`self.voiceMode`) :`NewEnumerator0` (make `VoiceSettings` null) :`NewEnumerator1` (make `VoiceSettings` (`self.DefaultSceneRoot`) "/Game/Titanfall_3/Data/SA_Positional.SA_Positional") :`NewEnumerator2` (make `VoiceSettings` null)) (`self.VOIPTalker`)))
    (:`Is Not Valid`
      (`KismetSystemLibrary.RetriggerableDelay` 0.2)
      (goto _label))))

(event `Server_SetVoiceMode`
  (params (voiceMode :type "/Game/Titanfall_3/Data/E_VoiceMode Enum" :default "NewEnumerator0"))
  (set `self.voiceMode` voiceMode))

(event `Key|H`
  (params (Key :type "Key Structure"))
  (:`Pressed`
    (`self.VOIPTalker`
      (:`then`
        (`self.Server_SetVoiceMode` "NewEnumerator1")
        (`AdvancedVoiceLibrary.StartNetworkedVoice` 0)
        (`KismetSystemLibrary.ExecuteConsoleCommand` "OSS.VoiceLoopback 1" (`PlayerState.GetPlayerController` (`self.PlayerState`)))
        (`KismetSystemLibrary.PrintString` "start'"))
      (:`else`)))
  (:`Released`
    (`AdvancedVoiceLibrary.StopNetworkedVoice` 0)
    (`self.Server_SetVoiceMode` "NewEnumerator0")))

(event `Key|J`
  (params (Key :type "Key Structure"))
  (:`Pressed`
    (`self.VOIPTalker`
      (:`then`
        (`self.Server_SetVoiceMode` "NewEnumerator2")
        (`AdvancedVoiceLibrary.StartNetworkedVoice` 0))
      (:`else`)))
  (:`Released`
    (`AdvancedVoiceLibrary.StopNetworkedVoice` 0)
    (`self.Server_SetVoiceMode` "NewEnumerator0")))

(event `Client_CloseVoiceLine`
  (`self.VOIPTalker`
    (:`then`
      (if (`|EnumInequality` (`self.voiceMode`) "NewEnumerator0")
        (`KismetSystemLibrary.ExecuteConsoleCommand` "ToggleSpeaking 0" (`PlayerState.GetPlayerController` (`self.PlayerState`))))
      (`AdvancedVoiceLibrary.MuteRemoteTalker` 0 (`AdvancedSessionsLibrary.GetUniqueNetIDFromPlayerState` (`self.PlayerState`)) true)
      (`AdvancedVoiceLibrary.RemoveAllRemoteTalkers`)
      (`VOIPLibrary.ClearVoicePackets` self))
    (:`else`)))

(event `self.ReceiveUnpossessed`
  (params (OldController :type "Controller Object Reference"))
  (`self.Client_CloseVoiceLine`))

(fn `OnRep_voiceMode`
  (set `VOIPTalker.Settings` (select `/Game/Titanfall_3/Data/E_VoiceMode` (`self.voiceMode`) :`NewEnumerator0` (make `VoiceSettings` null) :`NewEnumerator1` (make `VoiceSettings` (`self.DefaultSceneRoot`) "/Game/Titanfall_3/Data/SA_Positional.SA_Positional") :`NewEnumerator2` (make `VoiceSettings` null)) (`self.VOIPTalker`)))

(fn `UserConstructionScript`)