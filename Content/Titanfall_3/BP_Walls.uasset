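; BP_Walls is a wall actor that starts and stops wall running for actors tagged WallRun.
; Entering its Box sends a WallRun Start gameplay event to a tagged actor; leaving sends Stop to any actor, without the tag check.
; The Start payload carries a synthetic hit result as target data, with the wall's forward vector stored in Location and the normalized box-to-actor direction as both normals.
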(event `self.Box.OnComponentBeginOverlap`
  (params (OverlappedComponent :type "PrimitiveComponent Object Reference") (OtherActor :type "Actor Object Reference") (OtherComp :type "PrimitiveComponent Object Reference") (OtherBodyIndex :type Integer) (bFromSweep :type Boolean) (SweepResult :type "HitResult Structure (by ref)"))
  (bind _returnvalue (`KismetMathLibrary.Normal` (- (`self.K2_GetActorLocation` OtherActor) (`SceneComponent.K2_GetComponentLocation` (`self.Box`)))))
  (if (`self.ActorHasTag` OtherActor "WallRun")
    (`AbilitySystemBlueprintLibrary.SendGameplayEventToActor` OtherActor (struct :`TagName` "Event.ActivateAbility.WallRun.Start") (make `GameplayEventData` :`TargetData` (`AbilitySystemBlueprintLibrary.AbilityTargetDataFromHitResult` (`GameplayStatics.MakeHitResult` false false 0.0 0.0 (`self.GetActorForwardVector`) (0.0 0.0 0.0) _returnvalue _returnvalue))))))

(event `self.Box.OnComponentEndOverlap`
  (params (OverlappedComponent :type "PrimitiveComponent Object Reference") (OtherActor :type "Actor Object Reference") (OtherComp :type "PrimitiveComponent Object Reference") (OtherBodyIndex :type Integer))
  (`AbilitySystemBlueprintLibrary.SendGameplayEventToActor` OtherActor (struct :`TagName` "Event.ActivateAbility.WallRun.Stop")))

(fn `UserConstructionScript`)